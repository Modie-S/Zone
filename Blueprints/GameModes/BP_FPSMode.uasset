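; Game mode for an FPS round in which the player must destroy all drones before time runs out.
; BeginPlay creates the HUD, counts placed drones and locks player input until the warm-up countdown ends.
; Tick switches on SessionState to run the warm-up or match timer, turning the clock red near zero.
; DroneDestroyed, PlayerEliminated and timer expiry end the round with an announcement and disabled input.
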(event EventBeginPlay
  (Utilities|FlowControl|Sequence
    (:then_0
      ;[1 1 1] HUD
      (bind _returnvalue (UserInterface|CreateWidget "/Game/Blueprints/HUD/WBP_GameMode.WBP_GameMode_C"))
      (bind _output_get (Variables|Default|SetHUD _returnvalue))
      (UserInterface|Viewport|AddtoViewport _output_get 0)
      (Rendering|Components|TextRender|SetText (Variables|/Game/Blueprints/HUD/WBP_GameMode.WBP_GameMode_C|GetAnnouncement _output_get) "LOCK N' LOAD")
      (bind _format_time (CallFunction|TimeRemainingFormat))
      (Rendering|Components|TextRender|SetText (Variables|/Game/Blueprints/HUD/WBP_GameMode.WBP_GameMode_C|GetTime _output_get) _format_time))
    (:then_1
      ;[1 1 1] Set No of Drones
      (bind _outactors (Actor|GetAllActorsOfClass "/Game/Blueprints/Enemies/BP_Drone.BP_Drone_C"))
      (Variables|Default|SetNumber%20Of%20Drones (Utilities|Array|Length _outactors))
      (Rendering|Components|TextRender|SetText (Variables|/Game/Blueprints/HUD/WBP_GameMode.WBP_GameMode_C|GetEnemyCountdown (Variables|Default|GetHUD)) (Utilities|Text|ToText(Integer) (Utilities|Array|Length _outactors))))
    (:then_2
      ;[1 1 1] Disable input
      (CallFunction|DisablePlayerInput))))

(event EventTick
  (params (DeltaSeconds :type Float%20%28single-precision%29))
  (switch Utilities|FlowControl|Switch|SwitchonE_SessionState (Variables|Default|GetSession%20State)
    (:NewEnumerator0
      (CallFunction|UpdateWarmUpTimer))
    (:NewEnumerator1
      (CallFunction|UpdateGameTimer DeltaSeconds))))

(fn ConstructionScript)

(fn DroneDestroyed
  (bind _result (Math|Integer|DecrementInt (Variables|Default|GetNumber%20Of%20Drones))
    (:%20%20
      (Rendering|Components|TextRender|SetText (Variables|/Game/Blueprints/HUD/WBP_GameMode.WBP_GameMode_C|GetEnemyCountdown (Variables|Default|GetHUD)) (Utilities|Text|ToText(Integer) _result))
      (if (<= (Variables|Default|GetNumber%20Of%20Drones) 0)
        (CallFunction|PlayerWin)))))

(fn UpdateWarmUpTimer
  (bind _returnvalue (Utilities|Time|GetGameTimeinSeconds))
  (bind _warmup_time (Variables|Default|GetWarmUp%20Time))
  (bind _returnvalue_2 (- _warmup_time _returnvalue))
  (bind _returnvalue_3 (Class|KismetMathLibrary|FCeil64 _returnvalue_2))
  (Rendering|Components|TextRender|SetText (Variables|/Game/Blueprints/HUD/WBP_GameMode.WBP_GameMode_C|GetGameCountdown (Variables|Default|GetHUD)) (Utilities|Text|ToText(String) _returnvalue_3))
  (if (<= _returnvalue_3 0)
    (CallFunction|StartGame)))

(fn DisablePlayerInput
  (bind _returnvalue (Game|Player|GetPlayerPawn 0))
  (bind _asbp_fpscharacter (Utilities|Casting|CastToBP_FPSCharacter _returnvalue))
  (Variables|/Game/Blueprints/Character/BP_FPSCharacter.BP_FPSCharacter_C|SetFire%20Button%20Pressed _asbp_fpscharacter false)
  (Input|DisableInput _returnvalue 0))

(fn StartGame
  (bind _returnvalue (Game|Player|GetPlayerPawn 0))
  (bind _hud (Variables|Default|GetHUD))
  (Variables|Default|SetSession%20State "NewEnumerator1")
  (bind _asplayer_controller (Utilities|Casting|CastToPlayerController (Pawn|GetController _returnvalue)))
  (Input|EnableInput _returnvalue _asplayer_controller)
  (Rendering|Components|TextRender|SetText (Variables|/Game/Blueprints/HUD/WBP_GameMode.WBP_GameMode_C|GetGameCountdown _hud) "")
  (Rendering|Components|TextRender|SetText (Variables|/Game/Blueprints/HUD/WBP_GameMode.WBP_GameMode_C|GetAnnouncement _hud) ""))

(fn UpdateGameTimer
  (params (Delta%20Time :type Float%20%28double-precision%29))
  (Variables|Default|SetTime%20Left (- (Variables|Default|GetTime%20Left) Delta%20Time))
  (bind _format_time (CallFunction|TimeRemainingFormat))
  (Rendering|Components|TextRender|SetText (Variables|/Game/Blueprints/HUD/WBP_GameMode.WBP_GameMode_C|GetTime (Variables|Default|GetHUD)) _format_time)
  (if (<= (Variables|Default|GetTime%20Left) 1e+01)
    (Appearance|SetColorandOpacity (Variables|/Game/Blueprints/HUD/WBP_GameMode.WBP_GameMode_C|GetTime (Variables|Default|GetHUD)) (Utilities|Struct|MakeSlateColor "(R=1.000000,G=0.000000,B=0.000000,A=0.750000)") :!class /Script/UMG.TextBlock)
    (if (<= (Variables|Default|GetTime%20Left) 0.0)
      (CallFunction|OutOfTime))))

(fn OutOfTime
  (bind _hud (Variables|Default|GetHUD))
  (Variables|Default|SetSession%20State "NewEnumerator2")
  (Rendering|Components|TextRender|SetText (Variables|/Game/Blueprints/HUD/WBP_GameMode.WBP_GameMode_C|GetTime _hud) "00:00")
  (Rendering|Components|TextRender|SetText (Variables|/Game/Blueprints/HUD/WBP_GameMode.WBP_GameMode_C|GetAnnouncement _hud) "TIME'S UP...")
  (CallFunction|DisablePlayerInput))

(fn TimeRemainingFormat
  (bind _time_left (Variables|Default|GetTime%20Left))
  (bind _returnvalue (/ _time_left 6e+01))
  (bind _returnvalue_2 (Class|KismetMathLibrary|FFloor64 _returnvalue))
  (return (Utilities|Text|FormatText "{Minutes}:{Seconds}" (Utilities|Text|ToText(String) _returnvalue_2) (Utilities|Text|ToText(Float) (- (Variables|Default|GetTime%20Left) (Math|Conversions|ToInteger(Byte) (* _returnvalue_2 60))) "HalfToEven" false true 2 2 0 0))))

(fn PlayerWin
  (bind _asbp_fpscharacter (Utilities|Casting|CastToBP_FPSCharacter (Game|Player|GetPlayerPawn 0)))
  (if (> (Variables|/Game/Blueprints/Character/BP_FPSCharacter.BP_FPSCharacter_C|GetHealth _asbp_fpscharacter) 0.0)
    (Variables|Default|SetSession%20State "NewEnumerator4")
    (Rendering|Components|TextRender|SetText (Variables|/Game/Blueprints/HUD/WBP_GameMode.WBP_GameMode_C|GetAnnouncement (Variables|Default|GetHUD)) "ALL DRONES DESTROYED!")
    (CallFunction|DisablePlayerInput)))

(fn PlayerEliminated
  (bind _hud (Variables|Default|GetHUD))
  (Variables|Default|SetSession%20State "NewEnumerator3")
  (Rendering|Components|TextRender|SetText (Variables|/Game/Blueprints/HUD/WBP_GameMode.WBP_GameMode_C|GetAnnouncement _hud) "YOU WERE ELIMINATED")
  (Rendering|Components|TextRender|SetText (Variables|/Game/Blueprints/HUD/WBP_GameMode.WBP_GameMode_C|GetTime _hud) "00:00")
  (CallFunction|DisablePlayerInput))